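; BP_Enemy is an opponent actor that follows the height of BP_Ball along the Z axis.
; Each Tick looks up the ball, stores its location and calls SetDirection, then offsets the actor on local Z by MoveDir times MoveSpeed, without delta-time scaling or sweep.
; SetDirection repeats the same comparison in its nested branch, so the downward case is unreachable and the actor only moves up or stops.
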(event EventBeginPlay)

(event Collision|EventActorBeginOverlap
  (params (OtherActor :type Actor%20Object%20Reference)))

(event EventTick
  (params (DeltaSeconds :type Float%20%28single-precision%29))
  (bind _returnvalue (Actor|GetActorOfClass "/Game/BP_Ball.BP_Ball_C"))
  (Variables|Default|SettargetPosition (Transformation|GetActorLocation _returnvalue))
  (CallFunction|SetDirection)
  (Transformation|AddActorLocalOffset (Math|Vector|MakeVector 0.0 0.0 (* (Variables|Default|GetmoveDir) (Variables|Default|GetmoveSpeed))) false false))

(fn ConstructionScript)

(fn SetDirection
  (if (<= (.Z (Math|Vector|BreakVector (Transformation|GetActorLocation))) (.Z (Math|Vector|BreakVector (Variables|Default|GettargetPosition))))
    (Variables|Default|SetmoveDir 1)
    (elif (<= (.Z (Math|Vector|BreakVector (Transformation|GetActorLocation))) (.Z (Math|Vector|BreakVector (Variables|Default|GettargetPosition))))
      (Variables|Default|SetmoveDir -1)
      (else
        (Variables|Default|SetmoveDir 0)))))