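; Player Blueprint that moves vertically along its local Z axis from the Up/Down input axis.
; Each tick it offsets itself by MoveSpeed times the axis value, without sweep or delta-time scaling, and stores the truncated axis value in MoveDir.
; Overlapping an actor tagged Wall sets MoveSpeed to zero, and nothing in this Blueprint restores it.
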(event EventBeginPlay)

(event EventTick
  (params (DeltaSeconds :type Float%20%28single-precision%29))
  (bind _returnvalue (Input|AxisValues|GetUp/Down))
  (Transformation|AddActorLocalOffset (Math|Vector|MakeVector 0.0 0.0 (* (Variables|Default|GetmoveSpeed) _returnvalue)) false false)
  (Variables|Default|SetmoveDir (Math|Float|Truncate _returnvalue)))

(event Collision|EventActorBeginOverlap
  (params (OtherActor :type Actor%20Object%20Reference))
  (if (Actor|ActorHasTag OtherActor "Wall")
    (Variables|Default|SetmoveSpeed 0.0)))

(event Input|AxisEvents|InputAxisUp/Down
  (params (AxisValue :type Float%20%28single-precision%29)))

(fn ConstructionScript)