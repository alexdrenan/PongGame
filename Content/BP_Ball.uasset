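; Pong-style ball actor that bounces between BP_Player and BP_Enemy paddles and off BP_Wall actors using ProjectileMovement.
; Paddle overlaps add random Z spin biased by the paddle's MoveDir and reverse Y; wall overlaps reverse Z.
; Both reversals share a one-second cooldown.
; Each Tick, a Y at or below either paddle's teleports it to a fixed point, keeping only Y velocity.
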(event EventBeginPlay)

(event Collision|EventActorBeginOverlap
  (params (OtherActor :type Actor%20Object%20Reference))
  (bind _asbp_player (Utilities|Casting|CastToBP_Player OtherActor)
    (:then
      (CallFunction|HandleBounce (Variables|/Game/BP_Player.BP_Player_C|GetmoveDir _asbp_player)))
    (:CastFailed
      (bind _asbp_enemy (Utilities|Casting|CastToBP_Enemy OtherActor)
        (:then
          (CallFunction|HandleBounce (Variables|/Game/BP_Enemy.BP_Enemy_C|GetmoveDir _asbp_enemy)))
        (:CastFailed
          (Utilities|Casting|CastToBP_Wall OtherActor)
          (CallFunction|ReverseZ))))))

(event EventTick
  (params (DeltaSeconds :type Float%20%28single-precision%29))
  (bind _projectilemovement (Variables|Default|GetProjectileMovement))
  (Variables|Default|SettimeSinceReversed (+ (Variables|Default|GettimeSinceReversed) DeltaSeconds))
  (bind _outofbounds (CallFunction|IsOutOfBounds))
  (if _outofbounds
    (Transformation|SetActorLocation "980.000000,20.000000,910.000000" false true)
    (Variables|/Script/Engine.MovementComponent|SetVelocity _projectilemovement (Math|Vector|MakeVector 0.0 (.Y (Math|Vector|BreakVector (Variables|/Script/Engine.MovementComponent|GetVelocity _projectilemovement))) 0.0))))

(fn ConstructionScript)

(fn AddSpin
  (params (Spin :type Float%20%28single-precision%29))
  (Variables|/Script/Engine.MovementComponent|SetVelocity (Variables|Default|GetProjectileMovement) (+ (Math|Vector|MakeVector 0.0 0.0 Spin) (Variables|/Script/Engine.MovementComponent|GetVelocity (Variables|Default|GetProjectileMovement)))))

(fn ReverseY
  (if (>= (Variables|Default|GettimeSinceReversed) 1.0)
    (Variables|/Script/Engine.MovementComponent|SetVelocity (Variables|Default|GetProjectileMovement) (Math|Vector|MakeVector (.X (Math|Vector|BreakVector (Variables|/Script/Engine.MovementComponent|GetVelocity (Variables|Default|GetProjectileMovement)))) (* -1 (.Y (Math|Vector|BreakVector (Variables|/Script/Engine.MovementComponent|GetVelocity (Variables|Default|GetProjectileMovement))))) (.Z (Math|Vector|BreakVector (Variables|/Script/Engine.MovementComponent|GetVelocity (Variables|Default|GetProjectileMovement))))))
    (Variables|Default|SettimeSinceReversed 0.0)))

(fn ReverseZ
  (if (>= (Variables|Default|GettimeSinceReversed) 1.0)
    (Variables|/Script/Engine.MovementComponent|SetVelocity (Variables|Default|GetProjectileMovement) (Math|Vector|MakeVector (.X (Math|Vector|BreakVector (Variables|/Script/Engine.MovementComponent|GetVelocity (Variables|Default|GetProjectileMovement)))) (.Y (Math|Vector|BreakVector (Variables|/Script/Engine.MovementComponent|GetVelocity (Variables|Default|GetProjectileMovement)))) (* -1 (.Z (Math|Vector|BreakVector (Variables|/Script/Engine.MovementComponent|GetVelocity (Variables|Default|GetProjectileMovement)))))))
    (Variables|Default|SettimeSinceReversed 0.0)))

(fn IsOutOfBounds
  (bind _outactors (Actor|GetAllActorsOfClass "/Game/BP_Player.BP_Player_C"))
  (if (<= (.Y (Math|Vector|BreakVector (Transformation|GetActorLocation))) (.Y (Math|Vector|BreakVector (Transformation|GetActorLocation (Utilities|Array|Get(acopy) _outactors)))))
    _
    (else
      (bind _outactors_2 (Actor|GetAllActorsOfClass "/Game/BP_Enemy.BP_Enemy_C"))
      (if (<= (.Y (Math|Vector|BreakVector (Transformation|GetActorLocation))) (.Y (Math|Vector|BreakVector (Transformation|GetActorLocation (Utilities|Array|Get(acopy) _outactors_2)))))
        _
        (else
          (return false)))))
  (return true))

(fn HandleBounce
  (params (Selection :type Integer))
  (bind _returnvalue (Math|Random|RandomFloatinRange -5e+01 5e+01))
  (switch int Selection
    (:-1
      (CallFunction|AddSpin (+ _returnvalue -125.0)))
    (:0
      (CallFunction|AddSpin (Math|Random|RandomFloatinRange -15.0 15.0)))
    (:1
      (CallFunction|AddSpin (+ _returnvalue 125.0))))
  (CallFunction|ReverseY))